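; BP_camera is a security camera that sweeps back and forth and detects the first-person player.
; A self-repeating move event uses a FlipFlop to alternate between start and end rotations, easing the camera mesh there with MoveComponentTo and a delay between moves.
; Every tick, a debug-drawn line trace for Pawn objects runs forward from a separate trace component.
; A hit on the cached player only prints "caught".
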(event `self.ReceiveBeginPlay`
  ; move camera
  (`self.Move camera`)
  (bind _asbp_first_person_character (cast `/Game/StarterContent/FirstPerson/Blueprints/BP_FirstPersonCharacter` (`GameplayStatics.GetPlayerCharacter` 0)))
  (set `self.PlayerReference` _asbp_first_person_character))

(event `Move camera`
  (bind (_currentrotation_roll _currentrotation_pitch _currentrotation_yaw) (`KismetMathLibrary.BreakRotator` (`self.CurrentRotation`)))
  ; move camera
  (`/Engine/EditorBlueprintResources/StandardMacros.FlipFlop`
    (:`A`
      (set `self.CurrentRotation` (`self.EndRotation`)))
    (:`B`
      (set `self.CurrentRotation` (`self.StartRotation`))))
  (`KismetSystemLibrary.MoveComponentTo` (`self.SM_camera`) (0.0 0.0 0.0) (`KismetMathLibrary.MakeRotator` _currentrotation_roll _currentrotation_pitch _currentrotation_yaw) false false (`self.SpeedRotation`))
  (`KismetSystemLibrary.Delay` (`self.DelayRotation`))
  (`self.Move camera`))

(event `Detect`
  (bind _sm_linetrace (`self.SM_LineTrace`))
  (bind _returnvalue (`SceneComponent.K2_GetComponentLocation` _sm_linetrace))
  (bind _outhit (`KismetSystemLibrary.LineTraceSingleForObjects` :`Start` _returnvalue :`End` (+ _returnvalue (* (`KismetMathLibrary.GetForwardVector` (`SceneComponent.K2_GetComponentRotation` _sm_linetrace)) (`self.DetectDistance`))) :`ObjectTypes` (`|MakeArray` "ObjectTypeQuery3" :!type "EObjectTypeQuery Enum") :`DrawDebugType` "ForOneFrame" :`TraceHitColor` (struct :`R` 0.010199 :`B` 1.0 :`A` 1.0)))
  (if (== (`.HitActor` (`GameplayStatics.BreakHitResult` _outhit)) (`self.PlayerReference`))
    (`KismetSystemLibrary.PrintString` "caught")))

(event `self.ReceiveTick`
  (params (DeltaSeconds :type "Float (single-precision)"))
  (`self.Detect`))

(fn `UserConstructionScript`)