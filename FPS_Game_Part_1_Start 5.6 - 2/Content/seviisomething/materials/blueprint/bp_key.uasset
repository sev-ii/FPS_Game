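; BP_Key is a key pickup that stays hidden and non-collidable until no Bptarget actors remain in the level.
; Tick searches for targets every frame to set mesh visibility and collision, with a DoOnce explosion effect and sound for the reveal.
; When the player's BP_FirstPersonCharacter overlaps the revealed key, it sets that character's HasKey, plays a pickup sound and destroys itself.
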(event `self.ReceiveBeginPlay`
  ; Setup variables
  (bind _asbp_first_person_character (cast `/Game/StarterContent/FirstPerson/Blueprints/BP_FirstPersonCharacter` (`GameplayStatics.GetPlayerCharacter` 0)))
  (set `self.As BP First Person Character` _asbp_first_person_character))

(event `self.ReceiveTick`
  (params (DeltaSeconds :type "Float (single-precision)"))
  (bind _returnvalue (`SceneComponent.K2_GetComponentLocation` (`self.SM_Key`)))
  ;[0.01463 0.1211 0.15 0.5] Key visibility
  (bind _outactors (`GameplayStatics.GetAllActorsOfClass` "/Game/seviisomething/materials/blueprint/bp-target.bp-target_C"))
  (bind _returnvalue_2 (`KismetArrayLibrary.Array_Add` _outactors))
  (bind _output_get (set `self.AllTargetsDestroyed` (<= _returnvalue_2 0)))
  (`SceneComponent.SetVisibility` (`self.SM_Key`) _output_get false)
  (`self.SetActorEnableCollision` _output_get)
  ;[0.15 0.1498 0.01827 0.5] keyspawn fx
  (if (`self.AllTargetsDestroyed`)
    (`/Engine/EditorBlueprintResources/StandardMacros.DoOnce` false
      (:`Completed`
        (`NiagaraFunctionLibrary.SpawnSystemAtLocation` "/Niagara/DefaultAssets/Templates/Systems/SimpleExplosion.SimpleExplosion" _returnvalue)
        (`GameplayStatics.SpawnSoundAtLocation` "/Engine/VREditor/Sounds/UI/Teleport_Committed.Teleport_Committed" _returnvalue (struct) 1.0 1.0 0.0 null null)))))

(event `self.collision.OnComponentBeginOverlap`
  (params (OverlappedComponent :type "PrimitiveComponent Object Reference") (OtherActor :type "Actor Object Reference") (OtherComp :type "PrimitiveComponent Object Reference") (OtherBodyIndex :type Integer) (bFromSweep :type Boolean) (SweepResult :type "HitResult Structure (by ref)"))
  ;[0.01803 0.15 0.02137 0.5] pickup key
  (if (and (== OtherActor (`self.As BP First Person Character`)) (`self.AllTargetsDestroyed`))
    (set `/Game/StarterContent/FirstPerson/Blueprints/BP_FirstPersonCharacter.HasKey` true (`self.As BP First Person Character`))
    (`GameplayStatics.SpawnSoundAtLocation` "/Engine/VREditor/Sounds/UI/Camera_Shutter.Camera_Shutter" (`self.K2_GetActorLocation`) (struct) 1.0 1.0 0.0 null null)
    (`self.K2_DestroyActor`)))

(fn `UserConstructionScript`)