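; A shootable target actor that slides back and forth and destroys itself after taking enough hits.
; Tick moves it each frame along its normalized Direction by Speed, without scaling by delta time or sweeping.
; A looping timer started on BeginPlay reverses Direction every MovementDuration.
; Each Hit event subtracts one hit point and destroys the actor at zero.
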(event `self.ReceiveHit`
  (params (MyComp :type "PrimitiveComponent Object Reference") (Other :type "Actor Object Reference") (OtherComp :type "PrimitiveComponent Object Reference") (bSelfMoved :type Boolean) (HitLocation :type "Vector Structure") (HitNormal :type "Vector Structure") (NormalImpulse :type "Vector Structure") (Hit :type "HitResult Structure (by ref)"))
  (set `self.HitPoints` (- (`self.HitPoints`) 1))
  (if (<= (`self.HitPoints`) 0)
    (`self.K2_DestroyActor`)))

(event `self.ReceiveBeginPlay`
  ;[0.01995 0.1342 0.15 0.5] Flip target direction
  (`KismetSystemLibrary.K2_SetTimerDelegate` (delegate `FlipDirection`) (`self.MovementDuration`) true))

(event `FlipDirection`
  ;[0.01995 0.1342 0.15 0.5] Flip target direction
  (set `self.Direction` (* (`self.Direction`) -1.0)))

(event `self.ReceiveTick`
  (params (DeltaSeconds :type "Float (single-precision)"))
  ;[0.02471 0.02844 0.15 0.5] target movement
  (`self.K2_AddActorWorldOffset` (* (`KismetMathLibrary.Normal` (`self.Direction`)) (`self.Speed`))))

(fn `UserConstructionScript`)